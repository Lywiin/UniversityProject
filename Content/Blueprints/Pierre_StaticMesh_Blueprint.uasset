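; Blueprint that displays a random binary number and its decimal equivalent on text components.
; On BeginPlay it randomizes bit values, writes them to Bin1 through Bin4, then shows their weighted sum in Dec, with BinNum1 as the lowest bit.
; BinNum1 is rolled twice and BinNum2 never, so the second bit keeps its initial value.
; The construction script holds an unconnected copy of the bit logic.
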(event EventBeginPlay
  (Variables|Default|SetBinNum1 (Math|Random|RandomIntegerinRange 0 1))
  (Variables|Default|SetBinNum1 (Math|Random|RandomIntegerinRange 0 1))
  (Variables|Default|SetBinNum3 (Math|Random|RandomIntegerinRange 0 1))
  (Variables|Default|SetBinNum4 (Math|Random|RandomIntegerinRange 0 1))
  (Rendering|Components|TextRender|SetText (Variables|Default|GetBin1) (Utilities|Text|ToText(Integer) (Variables|Default|GetBinNum1)))
  (Rendering|Components|TextRender|SetText (Variables|Default|GetBin2) (Utilities|Text|ToText(Integer) (Variables|Default|GetBinNum2)))
  (Rendering|Components|TextRender|SetText (Variables|Default|GetBin3) (Utilities|Text|ToText(Integer) (Variables|Default|GetBinNum3)))
  (Rendering|Components|TextRender|SetText (Variables|Default|GetBin4) (Utilities|Text|ToText(Integer) (Variables|Default|GetBinNum4)))
  (bind _output_get (Variables|Default|SetDecNum (+ (Variables|Default|GetBinNum1) (* (Variables|Default|GetBinNum2) 2) (* (Variables|Default|GetBinNum3) 4) (* (Variables|Default|GetBinNum4) 8))))
  (Rendering|Components|TextRender|SetText (Variables|Default|GetDec) (Utilities|Text|ToText(Integer) _output_get)))

(fn ConstructionScript)